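; BP_SM is a plane actor that flies forward on its own while its left and right propellers spin.
; Each Tick rolls both propeller components around their local X axis by a Speed variable scaled by delta time.
; The same Tick offsets the actor along its local X axis at a fixed, frame-rate-independent rate, separate from the propeller Speed.
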(event EventTick
  (params (DeltaSeconds :type Float%20%28single-precision%29))
  (Variables|Default|SetSpeed2_0 (* (Variables|Default|GetSpeed) (Utilities|Time|GetWorldDeltaSeconds)))
  (Transformation|AddLocalRotation (Variables|Default|GetLeftPr) (Math|Rotator|MakeRotator (Variables|Default|GetSpeed2_0) 0.0 0.0) false false)
  (Transformation|AddLocalRotation (Variables|Default|GetRightPr) (Math|Rotator|MakeRotator (Variables|Default|GetSpeed2_0) 0.0 0.0) false false)
  (Transformation|AddActorLocalOffset (Math|Vector|MakeVector (* (Utilities|Time|GetWorldDeltaSeconds) 5e+01) 0.0 0.0) false false))

(fn ConstructionScript)